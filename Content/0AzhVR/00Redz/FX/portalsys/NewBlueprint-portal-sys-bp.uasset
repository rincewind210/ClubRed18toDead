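; Portal actor that teleports a vr-AzhCH character entering its capsule to its linked Target portal, keeping the player's control rotation.
; Before teleporting it calls HidePortal on the Target, which switches off that effect and blocks porting for one second to prevent bounce-back.
; End overlap calls ShowPortal, which re-enables porting at once but sets the effect inactive.
; The construction script captures a scene cube and feeds a color-and-cubemap dynamic material to the Portal effect.
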(event OnComponentBeginOverlap(Capsule)
  (params (OverlappedComponent :type Primitive%20Component%20Object%20Reference) (OtherActor :type Actor%20Object%20Reference) (OtherComp :type Primitive%20Component%20Object%20Reference) (OtherBodyIndex :type Integer) (bFromSweep :type Boolean) (SweepResult :type Hit%20Result%20Structure%20%28by%20ref%29))
  (bind _target (Variables|Default|Gettarget))
  (bind _asvr__azh_ch (Utilities|Casting|CastTovr-AzhCH OtherActor))
  (if (Variables|Default|Getcan-port)
    (Variables|Default|SetAs%20Vr-%20Azh%20CH _asvr__azh_ch)
    (CallFunction|HidePortal _target)
    (Utilities|FlowControl|Delay 0.02)
    (Default|Portal-to (Variables|Default|GetAs%20Vr-%20Azh%20CH) (Transformation|GetWorldLocation (Variables|NewBlueprint-portal-sys-bp_C|GetCapsule _target)) (Pawn|GetControlRotation (Game|GetPlayerController 0) :!class /Script/Engine.Controller))))

(event OnComponentEndOverlap(Capsule)
  (params (OverlappedComponent :type Primitive%20Component%20Object%20Reference) (OtherActor :type Actor%20Object%20Reference) (OtherComp :type Primitive%20Component%20Object%20Reference) (OtherBodyIndex :type Integer))
  (Utilities|Casting|CastTovr-AzhCH OtherActor)
  (CallFunction|ShowPortal))

(event Custom|hide%20portal
  (Components|Activation|Deactivate (Variables|Default|Getportal))
  (Variables|Default|Setcan-port false)
  (Utilities|FlowControl|Delay 1.0)
  (Components|Activation|SetActive (Variables|Default|Getportal) true false)
  (Variables|Default|Setcan-port true))

(event Custom|show%20portal
  (Components|Activation|SetActive (Variables|Default|Getportal) false false)
  (Variables|Default|Setcan-port true))

(event EventBeginPlay)

(event Collision|EventActorBeginOverlap
  (params (OtherActor :type Actor%20Object%20Reference)))

(event EventTick
  (params (DeltaSeconds :type Float%20%28single-precision%29)))

(fn ConstructionScript
  (Rendering|SceneCapture|CaptureScene (Variables|Default|GetSceneCaptureComponentCube) :!class /Script/Engine.SceneCaptureComponentCube)
  (bind _returnvalue (Rendering|Material|CreateDynamicMaterialInstance (Variables|Default|GetMaterial%20inst) "None" "None" :!class /Script/Engine.KismetMaterialLibrary))
  (Rendering|Material|SetVectorParameterValue _returnvalue "color" (Variables|Default|Getcolor) :!class /Script/Engine.MaterialInstanceDynamic)
  (Rendering|Material|SetTextureParameterValue _returnvalue "cubemapportal" (Variables|Default|Getmap))
  (Class|NiagaraComponent|SetVariableMaterial (Variables|Default|Getportal) "mic" _returnvalue))