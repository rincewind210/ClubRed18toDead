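; HDRI backdrop actor that projects a cubemap onto a size-scaled mesh and recaptures its skylight.
; Construction builds a dynamic material for camera or center projection, feeding it the cubemap, intensity, lighting distance, yaw and projection position.
; It flattens the scene component's rotation to yaw only.
; An unfinished random-cubemap cycle sets a looping timer on a random cubemap rather than the actor; setmap is empty and the skylight blend never runs.
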(fn ConstructionScript
  (Components|StaticMesh|SetStaticMesh (Variables|Components|GetGeometry) (Variables|HDRIBackdrop|GetMesh))
  (Transformation|SetWorldScale3D (Variables|Components|GetGeometry) (Math|Conversions|ToVector(Float) (/ (Variables|HDRIBackdrop|GetSize) (/ (.SphereRadius (Collision|GetComponentBounds (Variables|Components|GetGeometry))) 5e+01))))
  (CallFunction|CreateMaterial)
  (Class|SkyLightComponent|RecaptureSky (Variables|Default|GetSkylight))
  (Utilities|Time|SetTimerbyFunctionName (.OutItem (Utilities|Array|Random (Variables|Default|Getcubemaparray))) "setmap" (Variables|Default|GetIn%20Blend%20Fraction) true))

(fn CreateMaterial
  (bind _scenecomponent (Variables|Default|GetSceneComponent))
  (Utilities|FlowControl|Sequence
    (:then_0
      (if (Variables|HDRIBackdrop|GetUseCameraProjection)
        (bind _returnvalue (Rendering|Material|CreateDynamicMaterialInstance "/Game/0AzhVR/00Redz/HDRIBackdrop/Materials/MI_HDRI_CameraProjection.MI_HDRI_CameraProjection" "HDRI_MID" "None" :!class /Script/Engine.KismetMaterialLibrary))
        (bind _output_get (Variables|HDRIBackdrop|SetMaterialInstance _returnvalue))
        (else
          (bind _returnvalue_2 (Rendering|Material|CreateDynamicMaterialInstance "/Game/0AzhVR/00Redz/HDRIBackdrop/Materials/MI_HDRI_CenterProjection.MI_HDRI_CenterProjection" "HDRI_MID" "None" :!class /Script/Engine.KismetMaterialLibrary))
          (bind _output_get_2 (Variables|HDRIBackdrop|SetMaterialInstance _returnvalue_2))))
      (Rendering|Material|SetTextureParameterValue _output_get_2 "HDRI_Map" (Variables|HDRIBackdrop|GetCubemap))
      (Rendering|Material|SetScalarParameterValue (Variables|HDRIBackdrop|GetMaterialInstance) "LightingDistance" (* (Variables|HDRIBackdrop|GetSize) (Variables|HDRIBackdrop|GetLightingDistanceFactor) 1e+02) :!class /Script/Engine.MaterialInstanceDynamic)
      (Rendering|Material|SetScalarParameterValue (Variables|HDRIBackdrop|GetMaterialInstance) "HDRI_Angle" (* (.Yaw (Math|Rotator|BreakRotator (Transformation|GetWorldRotation (Variables|Default|GetSceneComponent)))) -1.0) :!class /Script/Engine.MaterialInstanceDynamic)
      (Rendering|Material|SetVectorParameterValue (Variables|HDRIBackdrop|GetMaterialInstance) "ProjectionPosition" (Math|Vector|MakeVector) :!class /Script/Engine.MaterialInstanceDynamic)
      (Rendering|Material|SetScalarParameterValue (Variables|HDRIBackdrop|GetMaterialInstance) "Intensity" (Variables|HDRIBackdrop|GetIntensity) :!class /Script/Engine.MaterialInstanceDynamic))
    (:then_1
      (Rendering|Material|SetMaterial (Variables|Components|GetGeometry) 0 (Variables|HDRIBackdrop|GetMaterialInstance))
      (Transformation|SetWorldRotation _scenecomponent (Math|Rotator|MakeRotator 0.0 0.0 (.yaw (Transformation|GetWorldRotation _scenecomponent))) false false))))

(fn Setmap)