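; Audio visualizer actor that plays a track and animates an equalizer, pulsing sphere and progress cube.
; BeginPlay gathers EQmesh_bp bars into an X-sorted array and starts the audio.
; Tick samples the hard-coded SoundWave's spectrum at game time, scaling bars and recolouring them and the sphere green, yellow or red by height.
; Audio component events drive sphere scale from envelope and cube height from playback percent.
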(event OnAudioPlaybackPercent(Audio)
  (params (PlayingSoundWave :type Sound%20Wave%20Object%20Reference) (PlaybackPercent :type Float%20%28single-precision%29))
  (Transformation|SetRelativeScale3D (Variables|Default|GetCube) (Math|Vector|MakeVector 1.0 1.0 (* PlaybackPercent 5.0))))

(event OnAudioSingleEnvelopeValue(Audio)
  (params (PlayingSoundWave :type Sound%20Wave%20Object%20Reference) (EnvelopeValue :type Float%20%28single-precision%29))
  (bind _sphere (Variables|Default|GetSphere))
  (bind _returnvalue (Transformation|GetWorldScale _sphere))
  (Transformation|SetRelativeScale3D (Variables|Default|GetSphere) (Math|Conversions|ToVector(Float) (* EnvelopeValue 15.0)))
  (if (> (.z _returnvalue) 0.5)
    (if (> (.z _returnvalue) 0.8)
      _)))

(event EventTick
  (params (DeltaSeconds :type Float%20%28single-precision%29))
  (bind _outspectrum (Class|SoundVisualizationStatics|CalculateFrequencySpectrum "/Game/0AzhVR/00Redz/audio/wavz/Dj_Redleg_A_Realm_Of_Sound_Master.Dj_Redleg_A_Realm_Of_Sound_Master" 0 (Utilities|Time|GetGameTimeinSeconds) 0.02 40))
  (Variables|Default|Setfrequencies3 _outspectrum)
  (for (_array_element _array_index) (Variables|Default|Getfbars3)
    (Transformation|SetActorScale3D _array_element (Math|Vector|MakeVector 1.0 1.0 (Math|Float|Clamp(Float) (/ (Utilities|Array|Get(acopy) (Variables|Default|Getfrequencies3) _array_index) 1e+01) 1.0 5e+03)))
    (if (> (.z (Transformation|GetActorScale3D _array_element)) 2.0)
      (if (> (.z (Transformation|GetActorScale3D _array_element)) 3.5)
        (Rendering|Material|SetMaterial (Variables|/Game/0AzhVR/Redz/EQmesh_bp.EQmesh_bp_C|GetStaticMesh _array_element) 0 "/Game/0AzhVR/00Redz/FX/EQspecAN/red_Inst_Inst_Inst.red_Inst_Inst_Inst")
        (else
          (Rendering|Material|SetMaterial (Variables|/Game/0AzhVR/Redz/EQmesh_bp.EQmesh_bp_C|GetStaticMesh _array_element) 0 "/Game/0AzhVR/00Redz/FX/EQspecAN/yelow_Inst_Inst.yelow_Inst_Inst")))
      (else
        (Rendering|Material|SetMaterial (Variables|/Game/0AzhVR/Redz/EQmesh_bp.EQmesh_bp_C|GetStaticMesh _array_element) 0 "/Game/0AzhVR/00Redz/FX/EQspecAN/green_Inst.green_Inst")))))

(event EventBeginPlay
  (bind _fbars3 (Variables|Default|Getfbars3))
  (bind _outactors (Actor|GetAllActorsOfClass "/Game/0AzhVR/Redz/EQmesh_bp.EQmesh_bp_C"))
  (for _array_element _outactors
    (bind (_array_element_2 _array_index) (Utilities|Array|ForEachLoopwithBreak _fbars3 :!label _label)
      (:LoopBody
        (if (not (< (.X (Math|Vector|BreakVector (Transformation|GetActorLocation _array_element_2))) (.X (Math|Vector|BreakVector (Transformation|GetActorLocation _array_element)))))
          (goto _label Break)))
      (:Completed
        (Utilities|Array|Insert _fbars3 _array_element _array_index)
        (Audio|Components|Audio|Play (Variables|Default|GetAudio) 0.0)))))

(fn ConstructionScript)