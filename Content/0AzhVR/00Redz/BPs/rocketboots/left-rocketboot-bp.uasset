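; Left rocket boot Blueprint that fixes itself to the player's VR character when play begins.
; On BeginPlay it casts player character 0 to vr-AzhCH and attaches to the left-rocketboot socket on its skeletal mesh, snapping location while keeping world rotation and relative scale.
; It then toggles the active state of three components, including a subtle emissive steam jet effect, with no thrust or movement logic.
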(event EventBeginPlay
  (bind _returnvalue (Game|GetPlayerCharacter 0))
  (Utilities|IsValid _returnvalue
    (:Is%20Valid
      (bind _asvr__azh_ch (Utilities|Casting|CastTovr-AzhCH _returnvalue))
      (Transformation|AttachComponentToComponent (Variables|/Game/0AzhVR/vr-azhCH.vr-AzhCH_C|GetSkeletalMeshik _asvr__azh_ch) "left-rocketboot" "SnapToTarget" "KeepWorld" "KeepRelative" true)
      (Components|Activation|ToggleActive (Variables|Default|GetP_Steam_Jet_Emissive_Subtle))
      (Components|Activation|ToggleActive (Variables|Default|Get%201))
      (Components|Activation|ToggleActive (Variables|Default|Get%20)))))

(fn ConstructionScript)